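; Player character for a swipe-controlled lane runner that moves forward automatically and manages a passenger meter.
; Tick detects a touch drag past a distance threshold and fires a DoOnce, re-armed on release, to classify the swipe direction.
; Horizontal swipes snap the capsule to the neighboring Tracks actor's location, while vertical swipes only print.
; BeginPlay adds the PassangerBar widget, and Tick drains PassangerMeter through a Delay, printing a warning when empty.
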(event `InputAction|swipe`
  (params (Key :type "Key Structure"))
  (bind (_locationx _locationy) (`PlayerController.GetInputTouchState` (`GameplayStatics.GetPlayerController` 0) "Touch1"))
  (bind _returnvalue (`KismetMathLibrary.MakeVector2D` _locationx _locationy))
  (bind (_x _y) (`KismetMathLibrary.BreakVector2D` (- (`self.TouchStart2DVector`) (`self.TouchEnd2DVector`))))
  (:`Pressed`
    (set `self.IsPressed` true)
    (set `self.TouchStart2DVector` _returnvalue))
  (:`Released`
    (set `self.IsPressed` false)
    (goto _label :!via `Reset`)))

(event `self.ReceiveTick`
  (params (DeltaSeconds :type "Float (single-precision)"))
  (bind (_locationx _locationy) (`PlayerController.GetInputTouchState` (`GameplayStatics.GetPlayerController` 0) "Touch1"))
  (bind _returnvalue (`KismetMathLibrary.MakeVector2D` _locationx _locationy))
  (bind (_x _y) (`KismetMathLibrary.BreakVector2D` (- (`self.TouchStart2DVector`) (`self.TouchEnd2DVector`))))
  (`|ExecutionSequence`
    (:`then_0`
      (if (> (`self.PassangerMeter`) 0)
        (`KismetSystemLibrary.Delay` 2.0)
        (bind _output_get (set `self.PassangerMeter` (- (`self.PassangerMeter`) 10)))
        (`KismetSystemLibrary.PrintString` (`KismetStringLibrary.Conv_IntToString` _output_get))
        (else
          (`KismetSystemLibrary.PrintString` "PassangersAreMad!"))))
    (:`then_1`
      (if (`self.IsPressed`)
        (if (> (`KismetMathLibrary.VSize2D` (- (`self.TouchStart2DVector`) _returnvalue)) 100.0)
          (`/Engine/EditorBlueprintResources/StandardMacros.DoOnce` false :!label _label
            (:`Completed`
              (set `self.TouchEnd2DVector` _returnvalue)
              (if (> (`KismetMathLibrary.Abs` _x) (`KismetMathLibrary.Abs` _y))
                (if (> _x 0.0)
                  (if (> (`self.CurrentTrack`) 0)
                    (set `self.CurrentTrack` (- (`self.CurrentTrack`) 1))
                    (`SceneComponent.K2_SetRelativeLocation` (`self.CapsuleComponent`) (`self.K2_GetActorLocation` (`|GetArrayItem` (`self.Tracks`) (`self.CurrentTrack`))) false false))
                  (elif (> (- (`KismetArrayLibrary.Array_Length` (`self.Tracks`)) 1) (`self.CurrentTrack`))
                    (set `self.CurrentTrack` (+ (`self.CurrentTrack`) 1))
                    (`SceneComponent.K2_SetRelativeLocation` (`self.CapsuleComponent`) (`self.K2_GetActorLocation` (`|GetArrayItem` (`self.Tracks`) (`self.CurrentTrack`))) false false)))
                (elif (> _y 0.0)
                  (`KismetSystemLibrary.PrintString` "SWIPED UP")
                  (else
                    (`KismetSystemLibrary.PrintString` "SWIPED DOWN")))))))))
    (:`then_2`
      (`PawnMovementComponent.AddInputVector` (`self.CharacterMovement`) (/ (`KismetMathLibrary.GetForwardVector` (struct)) 5.0) false))))

(event `self.ReceiveBeginPlay`
  (`|ExecutionSequence`
    (:`then_0`
      (bind _returnvalue (`|CreateWidget` "/Game/Blueprints/Target/PassangerBar.PassangerBar_C"))
      (`UserWidget.AddToViewport` _returnvalue 0))
    (:`then_1`
      (`SceneComponent.K2_SetRelativeLocation` (`self.CapsuleComponent`) (`self.K2_GetActorLocation` (`|GetArrayItem` (`self.Tracks`))) false false))))

(fn `UserConstructionScript`)