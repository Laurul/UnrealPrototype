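; Pawn that detects four-direction touch swipes and copies another pawn's camera position.
; The swipe input stores the touch start, and Tick fires a DoOnce beyond a drag threshold, re-armed on release.
; The dominant axis sets PressIndex and prints the direction, though down and left share an index.
; Tick also moves its camera to the PlayerPawn camera's location and prints it.
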(event `InputAction|swipe`
  (params (Key :type "Key Structure"))
  (bind (_locationx _locationy) (`PlayerController.GetInputTouchState` (`GameplayStatics.GetPlayerController` 0) "Touch1"))
  (bind _returnvalue (`KismetMathLibrary.MakeVector2D` _locationx _locationy))
  (bind (_x _y) (`KismetMathLibrary.BreakVector2D` (- (`self.TouchStart2DVector`) (`self.TouchEnd2DVector`))))
  (:`Pressed`
    (set `self.IsPressed` true)
    (set `self.TouchStart2DVector` _returnvalue))
  (:`Released`
    (set `self.IsPressed` false)
    (goto _label :!via `Reset`)))

(event `self.ReceiveTick`
  (params (DeltaSeconds :type "Float (single-precision)"))
  (bind _camera (`self.Camera`))
  (bind (_locationx _locationy) (`PlayerController.GetInputTouchState` (`GameplayStatics.GetPlayerController` 0) "Touch1"))
  (bind _returnvalue (`KismetMathLibrary.MakeVector2D` _locationx _locationy))
  (bind (_x _y) (`KismetMathLibrary.BreakVector2D` (- (`self.TouchStart2DVector`) (`self.TouchEnd2DVector`))))
  (`|ExecutionSequence`
    (:`then_0`
      (`|ExecutionSequence`
        (:`then_0`
          (if (`self.IsPressed`)
            (if (> (`KismetMathLibrary.VSize2D` (- (`self.TouchStart2DVector`) _returnvalue)) 100.0)
              (`/Engine/EditorBlueprintResources/StandardMacros.DoOnce` false :!label _label
                (:`Completed`
                  (set `self.TouchEnd2DVector` _returnvalue)
                  (if (> (`KismetMathLibrary.Abs` _x) (`KismetMathLibrary.Abs` _y))
                    (if (> _x 0.0)
                      (set `self.press index` 3)
                      (`KismetSystemLibrary.PrintString` "SWIEPED LEFT")
                      (else
                        (set `self.press index` 4)
                        (`KismetSystemLibrary.PrintString` "SWIPED RIGHT")))
                    (elif (> _y 0.0)
                      (set `self.press index` 1)
                      (`KismetSystemLibrary.PrintString` "SWIPED UP")
                      (else
                        (set `self.press index` 3)
                        (`KismetSystemLibrary.PrintString` "SWIPED DOWN")))))))))))
    (:`then_1`
      (`SceneComponent.K2_SetWorldLocation` _camera (`SceneComponent.K2_GetComponentLocation` (`PlayerPawn.Camera` (`self.playerPawn`))) false false)
      (`KismetSystemLibrary.PrintString` (`KismetStringLibrary.Conv_VectorToString` (`SceneComponent.K2_GetComponentLocation` _camera)) true true (struct :`G` 0.66 :`B` 1.0 :`A` 1.0) 20.0))))

(event `self.ReceiveBeginPlay`
  (`|ExecutionSequence`))

(fn `UserConstructionScript`)